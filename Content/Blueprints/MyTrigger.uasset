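; MyTrigger is a box trigger that calls a TriggerActivated dispatcher when an actor with a configured tag begins overlapping it.
; Events toggle whether it is enabled, and the DoOnce flag routes activation through a one-shot gate that ResetDoOnce re-arms, or lets it fire on every overlap.
; The construction script applies the configurable box extent and label text.
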(event OnComponentBeginOverlap(Box)
  (params (OverlappedComponent :type Primitive%20Component%20Object%20Reference) (OtherActor :type Actor%20Object%20Reference) (OtherComp :type Primitive%20Component%20Object%20Reference) (OtherBodyIndex :type Integer) (bFromSweep :type Boolean) (SweepResult :type Hit%20Result%20Structure%20%28by%20ref%29))
  (if (Actor|ActorHasTag OtherActor (Variables|Default|GetActorHasTagToActivate))
    (if (Variables|Default|GetEnabled)
      (if (Variables|Default|GetDoOnce)
        (Utilities|FlowControl|DoOnce false
          (:Completed
            _)))
      (Default|CallTriggerActivatedDispatcher))))

(event Custom|EnableTrigger
  (Variables|Default|SetEnabled true))

(event Custom|DisableTrigger
  (Variables|Default|SetEnabled false))

(event Custom|ResetDoOnce
  (Utilities|FlowControl|DoOnce false) ; enters at Reset
)

(fn ConstructionScript
  (Components|Box|SetBoxExtent (Variables|Default|GetBox) (Variables|Default|GetTriggerExtent) true)
  (Rendering|Components|TextRender|SetText (Variables|Default|GetTextRender) (Variables|Default|GetTriggerText)))