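; EnergyItem is a single-use pickup that restores energy to the player's ROV.
; When an actor tagged Player overlaps its Box, a DoOnce gate adds a fixed amount to the ROV's Energy, capped at the maximum.
; The ROV comes from casting player character 0 rather than the overlapping actor, and the item is then hidden, not destroyed.
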(event OnComponentBeginOverlap(Box)
  (params (OverlappedComponent :type Primitive%20Component%20Object%20Reference) (OtherActor :type Actor%20Object%20Reference) (OtherComp :type Primitive%20Component%20Object%20Reference) (OtherBodyIndex :type Integer) (bFromSweep :type Boolean) (SweepResult :type Hit%20Result%20Structure%20%28by%20ref%29))
  (bind _returnvalue (Game|GetPlayerCharacter 0))
  (bind _asrov (Utilities|Casting|CastToROV _returnvalue))
  (if (Actor|ActorHasTag OtherActor "Player")
    (Utilities|FlowControl|DoOnce false
      (:Completed
        (if (<= (Variables|/Game/ROV/ROV.ROV_C|GetEnergy _asrov) 9e+01)
          (Variables|/Game/ROV/ROV.ROV_C|SetEnergy _asrov (+ (Variables|/Game/ROV/ROV.ROV_C|GetEnergy _asrov) 1e+01))
          (else
            (Variables|/Game/ROV/ROV.ROV_C|SetEnergy _asrov 1e+02)))
        (Rendering|SetActorHiddenInGame true)))))

(event EventBeginPlay)

(event Collision|EventActorBeginOverlap
  (params (OtherActor :type Actor%20Object%20Reference)))

(event EventTick
  (params (DeltaSeconds :type Float%20%28single-precision%29)))

(fn ConstructionScript)