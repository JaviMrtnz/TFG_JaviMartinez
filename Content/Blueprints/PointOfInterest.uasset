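; Point of interest trigger volume that registers a visit on the ROV player character when a tagged actor enters it.
; While enabled, an overlap fires the activation dispatcher, activates a particle effect and prints the ROV's updated point count; the sound call has no sound assigned yet.
; An optional, resettable DoOnce limits it to one activation.
; The construction script applies the editable box extent and label text.
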(event OnComponentBeginOverlap(Box)
  (params (OverlappedComponent :type Primitive%20Component%20Object%20Reference) (OtherActor :type Actor%20Object%20Reference) (OtherComp :type Primitive%20Component%20Object%20Reference) (OtherBodyIndex :type Integer) (bFromSweep :type Boolean) (SweepResult :type Hit%20Result%20Structure%20%28by%20ref%29))
  (bind _returnvalue (Game|GetPlayerCharacter 0))
  (bind _asrov (Utilities|Casting|CastToROV _returnvalue))
  ;[0.05098 0.05098 0.05098] Trigger
  (if (Actor|ActorHasTag OtherActor (Variables|Default|GetActorHasTagToActivate))
    (if (Variables|Default|GetEnabled)
      (if (Variables|Default|GetDoOnce)
        (Utilities|FlowControl|DoOnce false
          (:Completed
            _)))
      (Default|CallTriggerActivatedDispatcher)
      (Components|Activation|Activate (Variables|Default|GetParticleSystem) false)
      ;;[0.05098 0.05098 0.05098] Falta añadir sonido
      (Audio|PlaySoundatLocation 0 (Transformation|GetActorLocation) "0, 0, 0" 1.0 1.0 0.0 0 0 0 0)
      (Default|PointVisited _asrov)
      (Development|PrintString (Utilities|String|ToString(Integer) (Variables|/Game/ROV/ROV.ROV_C|GetPointsCount _asrov))))))

(event Custom|EnableTrigger
  ;[0.05098 0.05098 0.05098] Trigger
  (Variables|Default|SetEnabled true))

(event Custom|DisableTrigger
  ;[0.05098 0.05098 0.05098] Trigger
  (Variables|Default|SetEnabled false))

(event Custom|ResetDoOnce
  (bind _returnvalue (Game|GetPlayerCharacter 0))
  (bind _asrov (Utilities|Casting|CastToROV _returnvalue))
  ;[0.05098 0.05098 0.05098] Trigger
  (Utilities|FlowControl|DoOnce false) ; enters at Reset
)

(fn ConstructionScript
  (Components|Box|SetBoxExtent (Variables|Default|GetBox) (Variables|Default|GetTriggerExtent) true)
  (Rendering|Components|TextRender|SetText (Variables|Default|GetTextRender) (Variables|Default|GetTriggerText)))